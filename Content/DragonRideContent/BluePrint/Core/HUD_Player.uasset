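; HUD_Player is a player HUD that displays a crosshair widget for dragon riding.
; On BeginPlay it caches the player pawn as a BP_DragonCharacter, then creates a WBP_DragonCrosshair and adds it to the viewport.
; Each Tick it passes the dragon's actor roll to the widget's update event, while its own UpdateCrosshair function is empty.
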(event `self.ReceiveBeginPlay`
  ;[0.4769 1 0.5228] Begin Play
  (`|ExecutionSequence`
    (:`then_0`
      (`self.InitPlayerVariable`))
    (:`then_1`
      (`self.InitCrosshairDragon`))))

(event `self.ReceiveTick`
  (params (DeltaSeconds :type "Float (single-precision)"))
  (bind _dragoncharacter (`self.DragonCharacter`))
  (bind _returnvalue_roll (`KismetMathLibrary.BreakRotator` (`self.K2_GetActorRotation` _dragoncharacter)))
  (`|ExecutionSequence`
    (:`then_0`
      (`/Engine/EditorBlueprintResources/StandardMacros.IsValid` _dragoncharacter
        (:`Is Valid`
          (`/Game/DragonRideContent/UMG/Widgets/Crosshair/Dragon/WBP_DragonCrosshair.CE_UpdateCrosshair` (`self.CrosshairDragonWidget`) _returnvalue_roll))))))

(fn `InitCrosshairDragon`
  (bind _returnvalue (`|CreateWidget` "/Game/DragonRideContent/UMG/Widgets/Crosshair/Dragon/WBP_DragonCrosshair.WBP_DragonCrosshair_C" (`GameplayStatics.GetPlayerController` 0)))
  (bind _output_get (set `self.CrosshairDragonWidget` _returnvalue))
  (`UserWidget.AddToViewport` _output_get 0))

(fn `InitPlayerVariable`
  (bind _asbp_dragon_character (cast `/Game/DragonRideContent/BluePrint/Characters/Dragons/BP_DragonCharacter` (`GameplayStatics.GetPlayerPawn` 0)))
  (set `self.DragonCharacter` _asbp_dragon_character))

(fn `UpdateCrosshair`)

(fn `UserConstructionScript`)